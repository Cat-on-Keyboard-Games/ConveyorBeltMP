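; Conveyor belt actor that pushes overlapping actors along its forward vector at a replicated Speed, with a dynamic material scaled to that speed.
; Optionally, characters skip the direct push and get one of three hidden-role FakeBase components by index, which the server slides along the belt as a movement base.
; Each base snaps under its character when out of range, and collision-ignore rules aim to pair it with that character alone.
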(event `self.ReceiveBeginPlay`
  (set `self.FakeBases` (`|MakeArray` (`self.FakeBase0`) (`self.FakeBase1`) (`self.FakeBase2`))))

(event `self.ReceiveTick`
  (params (DeltaSeconds :type "Float (single-precision)"))
  (`self.UpdateCharacters`)
  (`self.MoveOverlappingActors` DeltaSeconds)
  (if (`self.UseFakeBases`)
    (`self.MoveFakeBases` DeltaSeconds)))

(fn `GetFakeBaseForCharacter`
  (params (Character :type "Character Object Reference"))
  (returns (FakeBase :type "BoxComponent Object Reference"))
  (bind _fakebases (`self.FakeBases`))
  (bind _returnvalue (`KismetArrayLibrary.Array_Find` (`self.Characters`) Character))
  (if (`KismetArrayLibrary.Array_IsValidIndex` _fakebases _returnvalue)
    (return (`|GetArrayItem` _fakebases _returnvalue))
    (else
      (return null))))

(fn `MoveFakeBases`
  (params (DeltaTime :type "Float (double-precision)"))
  (locals (Character :type "Character Object Reference") (FakeBase :type "BoxComponent Object Reference") (CharacterLocationInLocalSpace :type "Vector Structure" :default (0.0 0.0 0.0)))
  (bind _characterlocationinlocalspace_x (`KismetMathLibrary.BreakVector` (`local.CharacterLocationInLocalSpace`)))
  (bind _returnvalue_x (`KismetMathLibrary.BreakVector` (`BoxComponent.GetUnscaledBoxExtent` (`local.FakeBase`))))
  (bind _relativelocation_x (`KismetMathLibrary.BreakVector` (`SceneComponent.RelativeLocation` (`local.FakeBase`))))
  (`/Engine/EditorBlueprintResources/ActorMacros.Switch Has Authority`
    (:`Authority`
      (for _array_element (`self.Characters`)
        (bind _output_get (set `local.Character` _array_element))
        (bind _fakebase (`self.GetFakeBaseForCharacter` _output_get))
        (bind _output_get_2 (set `local.FakeBase` _fakebase))
        (`/Engine/EditorBlueprintResources/StandardMacros.IsValid` _output_get_2
          (:`Is Valid`
            (if (`PrimitiveComponent.IsOverlappingActor` (`self.Box`) (`local.Character`))
              (`|ExecutionSequence`
                (:`then_0`
                  (bind _output_get_3 (set `local.CharacterLocationInLocalSpace` (`KismetMathLibrary.InverseTransformLocation` (`self.GetTransform`) (`self.K2_GetActorLocation` (`local.Character`)))))
                  (if (and (> (`KismetMathLibrary.Abs` (- (.x _output_get_3) _relativelocation_x)) (* _returnvalue_x 1.25)) (!= (`CharacterMovementComponent.GetMovementBase` (`Character.CharacterMovement` (`local.Character`))) (`local.FakeBase`)))
                    (`SceneComponent.K2_SetRelativeLocation` (`local.FakeBase`) (`KismetMathLibrary.MakeVector` _characterlocationinlocalspace_x 0.0 1.0) false false)))
                (:`then_1`
                  (`SceneComponent.K2_AddRelativeLocation` (`local.FakeBase`) (`KismetMathLibrary.MakeVector` (* (`local.DeltaTime`) (`self.Speed`))) false false))))))))
    (:`Remote`
      (return))))

(fn `MoveOverlappingActors`
  (params (DeltaTime :type "Float (double-precision)"))
  (for _array_element (`PrimitiveComponent.GetOverlappingActors` (`self.Box`) null)
    (if (!= _array_element self)
      (if (or (not (`self.UseFakeBases`)) (not (`GameplayStatics.ObjectIsA` _array_element "/Script/Engine.Character")))
        (`self.K2_AddActorWorldOffset` _array_element (* (`local.DeltaTime`) (`self.Speed`) (`self.GetActorForwardVector`)) true false)))))

(fn `OnRep_Speed`
  (`MaterialInstanceDynamic.SetScalarParameterValue` (`self.MaterialInstance`) "None" (* (`self.Speed`) (`self.MaterialSpeedMultiplier`))))

(fn `UpdateCharacters`
  (bind _outactors (`GameplayStatics.GetAllActorsOfClass` "/Script/Engine.Character"))
  (bind _output_get (set `self.Characters` _outactors))
  (for _array_element _output_get
    (bind _fakebase (`self.GetFakeBaseForCharacter` null))
    (`/Engine/EditorBlueprintResources/StandardMacros.IsValid` _fakebase
      (:`Is Valid`
        (for _array_element_2 (`self.Characters`)
          (bind _returnvalue (!= _array_element _array_element_2))
          (`PrimitiveComponent.IgnoreActorWhenMoving` _fakebase _array_element_2 _returnvalue)
          (`PrimitiveComponent.IgnoreComponentWhenMoving` (`Character.CapsuleComponent` _array_element_2) _fakebase _returnvalue))))))

(fn `UserConstructionScript`
  (bind _returnvalue (`PrimitiveComponent.CreateDynamicMaterialInstance` (`self.StaticMesh`) 1 null "None"))
  (bind _output_get (set `self.MaterialInstance` _returnvalue))
  (`MaterialInstanceDynamic.SetScalarParameterValue` _output_get "Speed" (* (`self.Speed`) (`self.MaterialSpeedMultiplier`)))
  (`MaterialInstanceDynamic.SetScalarParameterValue` _output_get "U Scale" (`self.MaterialScaleU`)))